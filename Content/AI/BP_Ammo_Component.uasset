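; Ammo component for the SWAT NPC that tracks its bullets and shares the count with its AI.
; The ammo widget, added to the viewport on BeginPlay, holds current and max ammo, which are copied to the owner's AI blackboard.
; Use1Bullet decrements the count and AddAmmo increases it, both updating the blackboard.
; AddAmmo resets overflow to a hardcoded 10 instead of MaxAmmo and prints the result.
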(event Custom|Use1Bullet
  (bind _result (Math|Integer|DecrementInt (Variables|/Game/Widgets/WBP_Ammo_Amount.WBP_Ammo_Amount_C|GetCurrentAmmo (Variables|Default|GetAmmoWidget)))
    (:%20%20
      (Class|BlackboardComponent|SetValueasInt (AI|GetBlackboard (AI|GetAIController (stale EventBeginPlay _asbp_swat_npc))) (Utilities|Name|MakeLiteralName "CurrentAmmo") _result))))

(event Custom|AddAmmo
  (params (Amount :type Integer))
  (bind _returnvalue (Utilities|Name|MakeLiteralName "CurrentAmmo"))
  (bind _ammowidget (Variables|Default|GetAmmoWidget))
  (bind _output_get (Variables|Default|SetNewAmmoAmount (+ Amount (Variables|/Game/Widgets/WBP_Ammo_Amount.WBP_Ammo_Amount_C|GetCurrentAmmo _ammowidget))))
  (if (> _output_get (Variables|/Game/Widgets/WBP_Ammo_Amount.WBP_Ammo_Amount_C|GetMaxAmmo _ammowidget))
    (Variables|Default|SetNewAmmoAmount 10))
  (Class|BlackboardComponent|SetValueasInt (AI|GetBlackboard (AI|GetAIController (stale EventBeginPlay _asbp_swat_npc))) _returnvalue (Variables|Default|GetNewAmmoAmount))
  (Variables|/Game/Widgets/WBP_Ammo_Amount.WBP_Ammo_Amount_C|SetCurrentAmmo (Variables|Default|GetAmmoWidget) (Variables|Default|GetNewAmmoAmount))
  (Development|PrintString (Utilities|String|ToString(Integer) (Class|BlackboardComponent|GetValueasInt (AI|GetBlackboard (AI|GetAIController (stale EventBeginPlay _asbp_swat_npc))) _returnvalue))))

(event EventBeginPlay
  (bind _ammowidget (Variables|Default|GetAmmoWidget))
  (UserInterface|Viewport|AddtoViewport (Variables|Default|GetAmmoWidget) 0)
  (bind _asbp_swat_npc (Utilities|Casting|CastToBP_SWAT_NPC (Components|GetOwner)))
  (Class|BlackboardComponent|SetValueasInt (AI|GetBlackboard (AI|GetAIController _asbp_swat_npc)) (Utilities|Name|MakeLiteralName "CurrentAmmo") (Variables|/Game/Widgets/WBP_Ammo_Amount.WBP_Ammo_Amount_C|GetCurrentAmmo _ammowidget))
  (Class|BlackboardComponent|SetValueasInt (AI|GetBlackboard (AI|GetAIController _asbp_swat_npc)) (Utilities|Name|MakeLiteralName "MaxAmmo") (Variables|/Game/Widgets/WBP_Ammo_Amount.WBP_Ammo_Amount_C|GetMaxAmmo _ammowidget)))

(event EventTick
  (params (DeltaSeconds :type Float%20%28single-precision%29)))